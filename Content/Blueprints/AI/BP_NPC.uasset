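; BP_NPC is a patrolling AI character that gets knocked into a ragdoll when it collides with the player's BP_Cart.
; The box overlap derives a horizontal direction away from the cart and launches both the mesh and a detached cart component with physics impulses.
; It then disables collision, unpossesses the controller and destroys the actor after a delay.
; Patrol functions serve the current route from an array, advancing and looping when one completes.
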(event `self.Box.OnComponentBeginOverlap`
  (params (OverlappedComponent :type "PrimitiveComponent Object Reference") (OtherActor :type "Actor Object Reference") (OtherComp :type "PrimitiveComponent Object Reference") (OtherBodyIndex :type Integer) (bFromSweep :type Boolean) (SweepResult :type "HitResult Structure (by ref)"))
  ;[0.6609 1 0.7316] On player collision
  (bind _asbp_cart (cast `/Game/Blueprints/Movement/BP_Cart` OtherActor))
  (bind (_returnvalue_x _returnvalue_y) (`KismetMathLibrary.BreakVector` (`KismetMathLibrary.Normal` (- (`self.K2_GetActorLocation` _asbp_cart) (`self.K2_GetActorLocation`)))))
  (`self.DoRagdoll` (`KismetMathLibrary.NegateVector` (`KismetMathLibrary.MakeVector` _returnvalue_x _returnvalue_y)))
  ;;[1 1 1] Queue for destruction
  (`KismetSystemLibrary.Delay` 3.0)
  (`self.K2_DestroyActor`))

(fn `DoRagdoll`
  (params (Direction :type "Vector Structure"))
  (locals (Impulse :type "Vector Structure"))
  (bind _returnvalue (`self.GetController`))
  (bind _mesh (`self.Mesh`))
  (bind _w (`self.w`))
  ;[0.6609 1 0.7316] Calculate impulse vector
  (set `local.Impulse` (* Direction (`self.ImpulsForce`)))
  (`|ExecutionSequence`
    (:`then_0`
      ;[0.6609 1 0.7316] Enable Physics & Launch Character
      (`PrimitiveComponent.SetSimulatePhysics` _mesh true)
      (`PrimitiveComponent.AddImpulse` _mesh (`local.Impulse`) "None" false))
    (:`then_1`
      ;[0.6609 1 0.7316] Enable Physics & Launch Cart
      (`PrimitiveComponent.SetSimulatePhysics` _w true)
      (`SceneComponent.K2_DetachFromComponent` _w "KeepWorld" "KeepWorld" "KeepWorld" false)
      (`PrimitiveComponent.AddImpulse` _w (`local.Impulse`) "None" false))
    (:`then_2`
      ;[0.6609 1 0.7316] Disable actor collisions & Unpossess
      (`PrimitiveComponent.SetCollisionEnabled` (`self.CapsuleComponent`) "NoCollision")
      (`PrimitiveComponent.SetCollisionEnabled` (`self.Box`) "NoCollision")
      (`/Engine/EditorBlueprintResources/StandardMacros.IsValid` _returnvalue
        (:`Is Valid`
          (`Controller.UnPossess` _returnvalue))))))

(fn `GetPatrolRoute`
  (returns (PatrolRoute :type "/Game/Blueprints/AI/BP_Route Object Reference"))
  (bind _output (`|GetArrayItem` (`self.RouteArr`) (`self.CurrentRouteIndex`)))
  (if (`/Game/Blueprints/AI/BP_Route.Completed` _output)
    (bind _route (`self.NextRoute`))
    (return _route)
    (else
      (return _output))))

(fn `NextRoute`
  (returns (Route :type "/Game/Blueprints/AI/BP_Route Object Reference"))
  (bind _result (`/Engine/EditorBlueprintResources/StandardMacros.IncrementInt` (`self.CurrentRouteIndex`))
    (:`  `
      (`|ExecutionSequence`
        (:`then_0`
          (if (>= _result (`KismetArrayLibrary.Array_Length` (`self.RouteArr`)))
            (set `self.CurrentRouteIndex` 0))
          (`/Game/Blueprints/AI/BP_Route.Restart` (`|GetArrayItem` (`self.RouteArr`) (`self.CurrentRouteIndex`))))
        (:`then_1`
          (return (`|GetArrayItem` (`self.RouteArr`) (`self.CurrentRouteIndex`))))))))

(fn `SetRouteArr`
  (params (RouteArr :type "Array of /Game/Blueprints/AI/BP_Route Object Reference"))
  (`KismetArrayLibrary.Array_Clear` (`self.RouteArr`))
  (for (_ _array_index) RouteArr
    (`KismetArrayLibrary.Array_Add` (`self.RouteArr`) (`|GetArrayItem` RouteArr _array_index))))

(fn `UserConstructionScript`)