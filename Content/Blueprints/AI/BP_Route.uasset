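; BP_Route is an AI route, likely for patrols, that tracks progress along the points of its Route spline.
; An increment event advances PatrolIndex and sets Completed once the index reaches or passes the spline point count.
; GetSplinePointAsWorld returns the world location of the current point, and Restart resets the index and completion flag.
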(event `IncrementPartolIndex`
  (bind _result (`/Engine/EditorBlueprintResources/StandardMacros.IncrementInt` (`self.PatrolIndex`))
    (:`  `
      (set `self.Completed` (>= _result (`SplineComponent.GetNumberOfSplinePoints` (`self.Route`)))))))

(fn `GetSplinePointAsWorld`
  (returns (Location :type "Vector Structure"))
  (return (`SplineComponent.GetLocationAtSplinePoint` (`self.Route`) (`self.PatrolIndex`) "World")))

(fn `Restart`
  (set `self.PatrolIndex` 0)
  (set `self.Completed` false))

(fn `UserConstructionScript`)