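; Item pickup manager component that holds a capacity-limited inventory of enum item IDs.
; AddItem stores an ID only when CanAddItem finds room under MaxCapacity, otherwise a capacity-full message is printed.
; RemoveItem checks for the ID, removes matches and prints the enum name.
; RemoveAll calls RemoveItem while looping over the items, but returns after the first element.
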(fn `AddItem`
  (params (ItemID :type "/Game/Items/ENUM_ItemID Enum" :default "NewEnumerator0"))
  (if (`self.CanAddItem`)
    (`KismetArrayLibrary.Array_Add` (`self.Items`) ItemID)
    (return)
    (else
      (return))))

(fn `CanAddItem`
  (returns (CanAdd :type Boolean))
  (if (< (`KismetArrayLibrary.Array_Length` (`self.Items`)) (`self.MaxCapacity`))
    (return true)
    (else
      (`KismetSystemLibrary.PrintString` "CANNOT ADD ITEM, \nCAPACITY FULL")
      (return false))))

(fn `RemoveAll`
  (for _array_element (`self.Items`)
    (`self.RemoveItem` _array_element)
    (return)))

(fn `RemoveItem`
  (params (ItemId :type "/Game/Items/ENUM_ItemID Enum" :default "NewEnumerator0"))
  (locals (LocalItemID :type "/Game/Items/ENUM_ItemID Enum" :default "NewEnumerator0"))
  (bind _output_get (set `local.LocalItemID` ItemId))
  (if (`KismetArrayLibrary.Array_Contains` (`self.Items`) _output_get)
    (for _array_element (`self.Items`)
      (if (`|EnumEquality` _array_element (`local.LocalItemID`))
        (bind _returnvalue (`KismetArrayLibrary.Array_RemoveItem` (`self.Items`) _array_element))
        (if _returnvalue
          (`KismetSystemLibrary.PrintString` (`KismetStringLibrary.Concat_StrStr` "ITEM REMOVED: " (`|GetEnumeratorNameAsString` (`local.LocalItemID`)))))))))