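; Actor component that generates a randomized to-do list of items, each with a required amount.
; On BeginPlay it gathers rows from DT_ItemDataTable, builds a random pool of item IDs with possible repeats, then fills the list from it.
; Each pick shrinks the pool at a separately rolled index, so the removed entry may differ from the picked one.
; EmptyToDoList clears the list, fires OnComplete and refills while the pool has items.
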(event `self.ReceiveBeginPlay`
  (bind _listtotakefrom (`self.FillListToTakeFrom`))
  (`self.FillToDoList` _listtotakefrom 3))

(fn `EmptyToDoList`
  (bind _listtotakefrom (`self.ListToTakeFrom`))
  (`KismetArrayLibrary.Array_Clear` (`self.ToDoList`))
  (`self.OnComplete`)
  (if (> (`KismetArrayLibrary.Array_Length` _listtotakefrom) 0)
    (`self.FillToDoList` _listtotakefrom 2)))

(fn `FillListToTakeFrom`
  (returns (ListToTakeFrom :type "Array of /Game/Items/ENUM_ItemID Enum"))
  (locals (AmountItemsInList :type Integer :default 20) (AllItems :type "Array of /Game/Blueprints/BPS_ItemData Structure"))
  (bind _output_itemid (break `/Game/Blueprints/BPS_ItemData` (`|GetArrayItem` (`local.AllItems`) (`KismetMathLibrary.RandomInteger` (`KismetArrayLibrary.Array_Length` (`local.AllItems`))))))
  (bind _outrownames (`DataTableFunctionLibrary.GetDataTableRowNames` "/Game/Blueprints/DT_ItemDataTable.DT_ItemDataTable"))
  (for _array_element _outrownames
    (bind _returnvalue (`|GetDataTableRow` "/Game/Blueprints/DT_ItemDataTable.DT_ItemDataTable" _array_element)
      (:`then`
        (`KismetArrayLibrary.Array_AddUnique` (`local.AllItems`) _returnvalue))))
  (for _ (range (`local.AmountItemsInList`))
    (`KismetArrayLibrary.Array_Add` (`self.ListToTakeFrom`) _output_itemid))
  (`KismetSystemLibrary.PrintString` (`KismetStringLibrary.Concat_StrStr` "AMOUNT: " (`KismetStringLibrary.Conv_IntToString` (`KismetArrayLibrary.Array_Length` (`self.ListToTakeFrom`)))))
  (return (`self.ListToTakeFrom`)))

(fn `FillToDoList`
  (params (ListToTakeFrom :type "Array of /Game/Items/ENUM_ItemID Enum") (AmountItemsToTake :type Integer))
  (locals (LocalAmountToTake :type Integer))
  (bind _returnvalue (`KismetArrayLibrary.Array_Length` ListToTakeFrom))
  (bind _listtotakefrom (`self.ListToTakeFrom`))
  (bind _returnvalue_2 (`KismetMathLibrary.RandomInteger` (`KismetArrayLibrary.Array_Length` _listtotakefrom)))
  (bind _output_get (set `local.LocalAmountToTake` AmountItemsToTake))
  (if (< _returnvalue _output_get)
    (set `local.LocalAmountToTake` _returnvalue))
  (for _ (range (`local.LocalAmountToTake`))
    (`KismetArrayLibrary.Array_AddUnique` (`self.ToDoList`) (make `/Game/Blueprints/BPS_ToDoItem` (`|GetArrayItem` _listtotakefrom _returnvalue_2) (+ (`KismetMathLibrary.RandomInteger` 3) 1)))
    (`KismetArrayLibrary.Array_Remove` (`self.ListToTakeFrom`) _returnvalue_2))
  (`KismetSystemLibrary.PrintString` "TO DO LIST CONTAINS" true true (struct :`G` 0.66 :`B` 1.0 :`A` 1.0) 10.0 "1")
  (for _array_element (`self.ToDoList`)
    (`KismetSystemLibrary.PrintString` (`KismetStringLibrary.Concat_StrStr` (`|GetEnumeratorNameAsString` (break `/Game/Blueprints/BPS_ToDoItem` _array_element)) "AMOUNT NEEDED:" (`KismetStringLibrary.Conv_IntToString` (`.AmountNeeded_5_13827824415953CB25F403BB9B545F88` (break `/Game/Blueprints/BPS_ToDoItem` _array_element)))) true true (struct :`G` 0.66 :`B` 1.0 :`A` 1.0) 10.0)))