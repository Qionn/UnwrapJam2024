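; BP_ItemActor is a world item pickup that takes on a random item type from DT_ItemDataTable.
; The construction script picks a random ItemID from the table's row count, looks up that row by enum name, and sets the mesh and weight.
; On box overlap, it calls AddItem on the other actor's BPC_ItemPickUpManager, passing a fixed enum value rather than ItemID.
; Actors without that component trigger a debug message.
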(event `self.Box.OnComponentBeginOverlap`
  (params (OverlappedComponent :type "PrimitiveComponent Object Reference") (OtherActor :type "Actor Object Reference") (OtherComp :type "PrimitiveComponent Object Reference") (OtherBodyIndex :type Integer) (bFromSweep :type Boolean) (SweepResult :type "HitResult Structure (by ref)"))
  (bind _returnvalue (`self.GetComponentByClass` OtherActor "/Game/Blueprints/BPC_ItemPickUpManager.BPC_ItemPickUpManager_C"))
  (`/Engine/EditorBlueprintResources/StandardMacros.IsValid` _returnvalue
    (:`Is Valid`
      (`/Game/Blueprints/BPC_ItemPickUpManager.AddItem` _returnvalue "NewEnumerator0"))
    (:`Is Not Valid`
      (`KismetSystemLibrary.PrintString` "No Item Pickup Component detected"))))

(fn `UserConstructionScript`
  (bind _outrownames (`DataTableFunctionLibrary.GetDataTableRowNames` "/Game/Blueprints/DT_ItemDataTable.DT_ItemDataTable"))
  (set `self.ItemID` (cast `/Game/Items/ENUM_ItemID` (`KismetMathLibrary.Conv_IntToByte` (`KismetMathLibrary.RandomInteger` (`KismetArrayLibrary.Array_Length` _outrownames)))))
  (bind _returnvalue (`|GetDataTableRow` "/Game/Blueprints/DT_ItemDataTable.DT_ItemDataTable" (`KismetStringLibrary.Conv_StringToName` (`|GetEnumeratorNameAsString` (`self.ItemID`))))
    (:`then`
      (bind _output_get (set `self.Mesh` (`self.Mesh`)))
      (bind (_itemid _mesh _weight) (break `/Game/Blueprints/BPS_ItemData` _returnvalue))
      (`StaticMeshComponent.SetStaticMesh` _output_get _mesh)
      (set `self.Weight` _weight))))