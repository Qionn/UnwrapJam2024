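; BP_MovableBase is a base actor for props that get knocked loose and removed when hit by a BP_Cart.
; On that hit, its static mesh starts simulating physics and takes a normalized impulse pointing away from the cart.
; A Niagara effect moves to the impact point at the cart's height and activates, then the actor destroys itself after a short delay.
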(event `self.StaticMesh.OnComponentHit`
  (params (HitComponent :type "PrimitiveComponent Object Reference") (OtherActor :type "Actor Object Reference") (OtherComp :type "PrimitiveComponent Object Reference") (NormalImpulse :type "Vector Structure") (Hit :type "HitResult Structure (by ref)"))
  (bind _staticmesh (`self.StaticMesh`))
  (bind _asbp_cart (cast `/Game/Blueprints/Movement/BP_Cart` OtherActor))
  (`|ExecutionSequence`
    (:`then_0`
      (`PrimitiveComponent.SetSimulatePhysics` _staticmesh true)
      (`PrimitiveComponent.AddImpulse` _staticmesh (`KismetMathLibrary.Normal` (- (`self.K2_GetActorLocation`) (`self.K2_GetActorLocation` _asbp_cart))) "None" false))
    (:`then_1`
      (bind (_returnvalue_x _returnvalue_y _returnvalue_z) (`KismetMathLibrary.BreakVector` (`self.K2_GetActorLocation` _asbp_cart)))
      (`SceneComponent.K2_SetWorldLocation` (`self.Niagara`) (`KismetMathLibrary.MakeVector` (.x Hit_Location) (.y Hit_Location) _returnvalue_z) false false)
      (`ActorComponent.SetActive` (`self.Niagara`) true false)
      (`KismetSystemLibrary.Delay` 3.0)
      (`self.K2_DestroyActor`))))

(fn `UserConstructionScript`)