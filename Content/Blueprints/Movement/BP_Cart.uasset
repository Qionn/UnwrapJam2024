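; BP_Cart is a cart that constantly drives forward, with Enhanced Input horizontal steering and a drift feel.
; Held input sets a target yaw step from DriftCurve sampled by hold time, plus a visual mesh angle; release zeroes both.
; Tick eases toward both targets, adding the yaw every frame without delta-time scaling, rotating the mesh separately, and moving the actor forward without sweep.
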(event `self.ReceiveTick`
  (params (DeltaSeconds :type "Float (single-precision)"))
  ;[0.7176 1 0.7686] Apply Rotation
  (bind _output_get (set `self.CurrentRotation` (`KismetMathLibrary.Lerp` (`self.CurrentRotation`) (`self.TargetRotation`) (* DeltaSeconds (`self.DriftResponsiveness`)))))
  (`self.K2_AddActorLocalRotation` (`KismetMathLibrary.MakeRotator` 0.0 0.0 _output_get))
  ;[0.7176 1 0.7686] Apply  Forward Velocity
  (`self.K2_AddActorWorldOffset` (* (`self.GetActorForwardVector`) (`self.ForwardSpeed`) (`GameplayStatics.GetWorldDeltaSeconds`)))
  ;[0.7176 1 0.7686] Apply Drift Animation
  (bind _output_get_2 (set `self.CurrentAnimRotation` (`KismetMathLibrary.Lerp` (`self.CurrentAnimRotation`) (`self.TargetAnimRotation`) (* (`GameplayStatics.GetWorldDeltaSeconds`) (`self.DriftResponsiveness`)))))
  (`SceneComponent.K2_SetRelativeRotation` (`self.StaticMesh`) (`KismetMathLibrary.MakeRotator` 0.0 0.0 _output_get_2) false false))

(event `EnhancedInput|/Game/Blueprints/Input/IA_Horizontal`
  (params (ActionValue :type "Float (double-precision)") (ElapsedSeconds :type "Float (double-precision)") (TriggeredSeconds :type "Float (double-precision)") (InputAction :type "InputAction Object Reference" :default "/Game/Blueprints/Input/IA_Horizontal.IA_Horizontal"))
  ;[0.7176 1 0.7686] Rotation Input
  (:`Triggered`
    (set `self.TargetAnimRotation` (* (`self.AnimationRotation`) ActionValue))
    (set `self.TargetRotation` (* ActionValue (`CurveFloat.GetFloatValue` (`self.DriftCurve`) TriggeredSeconds) (`self.DriftAmplification`))))
  (:`Completed`
    ;;[1 1 1] Reset States
    (set `self.TargetRotation` 0.0)
    (set `self.TargetAnimRotation` 0.0)))

(fn `UserConstructionScript`)