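; BP_CartWheelComponent is a cart wheel component that turns itself to face the direction it is travelling.
; It stores its world location on BeginPlay, then each Tick derives a normalized direction from the change since the previous position.
; It zeroes that vector's Z so the resulting world rotation follows only horizontal heading, then saves the current location for the next frame.
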(event `self.ReceiveBeginPlay`
  ;[0.6392 1 0.7176] Get Starting Location
  (set `self.PreviousPosition` (`self.K2_GetComponentLocation`)))

(event `self.ReceiveTick`
  (params (DeltaSeconds :type "Float (single-precision)"))
  (bind (_returnvalue_x _returnvalue_y) (`KismetMathLibrary.BreakVector` (`KismetMathLibrary.Normal` (`KismetMathLibrary.Normal` (- (`self.K2_GetComponentLocation`) (`self.PreviousPosition`))))))
  ;[0.6392 1 0.7176] Set Rotation
  (`self.K2_SetWorldRotation` (`KismetMathLibrary.Conv_VectorToRotator` (`KismetMathLibrary.MakeVector` _returnvalue_x _returnvalue_y)))
  ;[0.6392 1 0.7176] Update Previous Location
  (set `self.PreviousPosition` (`self.K2_GetComponentLocation`)))