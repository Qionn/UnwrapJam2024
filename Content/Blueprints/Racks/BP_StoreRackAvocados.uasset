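; Store rack actor that gives an item to actors overlapping its box and shows that item on placeholder meshes.
; On BeginPlay it refills to MaxItems and randomly picks a DT_ItemDataTable row matching its RackType, though the random range skips the last match.
; Each overlap calls AddItem on the actor's BPC_ItemPickUpManager and decrements stock.
; At zero it clears the meshes, but overlaps still grant items.
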(event `self.ReceiveBeginPlay`
  (`self.InitStoreRack`))

(event `self.Box.OnComponentBeginOverlap`
  (params (OverlappedComponent :type "PrimitiveComponent Object Reference") (OtherActor :type "Actor Object Reference") (OtherComp :type "PrimitiveComponent Object Reference") (OtherBodyIndex :type Integer) (bFromSweep :type Boolean) (SweepResult :type "HitResult Structure (by ref)"))
  (bind _itemdata_itemid (break `/Game/Blueprints/BPS_ItemData` (`self.ItemData`)))
  (`/Game/Blueprints/BPC_ItemPickUpManager.AddItem` (`self.GetComponentByClass` OtherActor "/Game/Blueprints/BPC_ItemPickUpManager.BPC_ItemPickUpManager_C") _itemdata_itemid)
  (bind _output_get (set `self.CurrentItems` (- (`self.CurrentItems`) 1)))
  (if (<= _output_get 0)
    (for _array_element (`SceneComponent.GetChildrenComponents` (`self.PlaceHolderParent`) true)
      (bind _asstatic_mesh_component (cast `StaticMeshComponent` _array_element))
      (`StaticMeshComponent.SetStaticMesh` _asstatic_mesh_component null))))

(fn `GetDataRowsByRackType`
  (params (`Rack Type` :type "/Game/Items/StoreRack/ENUM_StoreRacks Enum" :default "NewEnumerator0"))
  (returns (DataRowsByRackType :type "Array of Name"))
  (locals (LocalRackType :type "/Game/Items/StoreRack/ENUM_StoreRacks Enum") (FilteredDataRows :type "Array of Name"))
  (bind _filtereddatarows (`local.FilteredDataRows`))
  (set `local.LocalRackType` `Rack Type`)
  (bind _outrownames (`DataTableFunctionLibrary.GetDataTableRowNames` "/Game/Blueprints/DT_ItemDataTable.DT_ItemDataTable"))
  (for _array_element _outrownames
    (bind _returnvalue (`|GetDataTableRow` "/Game/Blueprints/DT_ItemDataTable.DT_ItemDataTable" _array_element)
      (:`then`
        (bind (_itemid _mesh _weight _storeracktype) (break `/Game/Blueprints/BPS_ItemData` _returnvalue))
        (if (`|EnumEquality` _storeracktype (`local.LocalRackType`))
          (bind _returnvalue_2 (`KismetArrayLibrary.Array_AddUnique` _filtereddatarows (`KismetStringLibrary.Conv_StringToName` (`|GetEnumeratorNameAsString` _itemid))))
          (`KismetSystemLibrary.PrintString` (`KismetStringLibrary.Conv_NameToString` (`|GetArrayItem` _filtereddatarows _returnvalue_2)))))))
  (return (`local.FilteredDataRows`)))

(fn `InitStoreRack`
  (locals (selectedItem :type Name))
  (set `self.CurrentItems` (`self.MaxItems`))
  (bind _datarowsbyracktype (`self.GetDataRowsByRackType` (`self.RackType`)))
  (bind _output_get (set `local.selectedItem` (`|GetArrayItem` _datarowsbyracktype (`KismetMathLibrary.RandomInteger` (- (`KismetArrayLibrary.Array_Length` _datarowsbyracktype) 1)))))
  (bind _returnvalue (`|GetDataTableRow` "/Game/Blueprints/DT_ItemDataTable.DT_ItemDataTable" _output_get)
    (:`then`
      (set `self.ItemData` _returnvalue)
      (for _array_element (`SceneComponent.GetChildrenComponents` (`self.PlaceHolderParent`) false)
        (bind _asstatic_mesh_component (cast `StaticMeshComponent` _array_element)
          (:`then`
            (`StaticMeshComponent.SetStaticMesh` _asstatic_mesh_component (`.Mesh_7_27A147C645E1759CE9F88AA5EAEEA84C` (break `/Game/Blueprints/BPS_ItemData` (`self.ItemData`)))))
          (:`CastFailed`
            (`KismetSystemLibrary.PrintString` "seli hweiughrgr")))))
    (:`RowNotFound`
      (`KismetSystemLibrary.PrintString` "row not found "))))

(fn `UserConstructionScript`
  (locals (SelectedItem :type Name)))