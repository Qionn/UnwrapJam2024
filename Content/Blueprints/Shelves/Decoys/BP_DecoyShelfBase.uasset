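; Base decoy shelf that displays a chosen item as instanced static meshes for visual dressing.
; The construction script looks up the Item enum's name in DT_ItemDataTable and applies that row's mesh to InstancedVisualItems.
; It then gives each existing instance a random yaw scaled by RotationVariaty, keeping location and scale, and applies all transforms in one batch update.
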(fn `UserConstructionScript`
  (locals (InstanceTransforms :type "Array of Transform Structure"))
  ;[0.6531 1 0.7187] Set visual item
  (bind _returnvalue (`|GetDataTableRow` "/Game/Blueprints/DT_ItemDataTable.DT_ItemDataTable" (`KismetStringLibrary.Conv_StringToName` (`|GetEnumeratorNameAsString` (`self.Item`))))
    (:`then`
      (`StaticMeshComponent.SetStaticMesh` (`self.InstancedVisualItems`) (`.Mesh_7_27A147C645E1759CE9F88AA5EAEEA84C` (break `/Game/Blueprints/BPS_ItemData` _returnvalue)))
      (for _index (range (`InstancedStaticMeshComponent.GetInstanceCount` (`self.InstancedVisualItems`)))
        (bind _outinstancetransform (`InstancedStaticMeshComponent.GetInstanceTransform` (`self.InstancedVisualItems`) _index false))
        ;[0.6531 1 0.7187] Populate transform array
        (`KismetArrayLibrary.Array_Add` (`local.InstanceTransforms`) (`KismetMathLibrary.MakeTransform` (.location _outinstancetransform) (`KismetMathLibrary.MakeRotator` 0.0 0.0 (`KismetMathLibrary.RandomFloatInRange` 0.0 (* (`self.RotationVariaty`) 360.0))) (.scale _outinstancetransform))))
      ;[0.6531 1 0.7187] Update instance transforms
      (`InstancedStaticMeshComponent.BatchUpdateInstancesTransforms` (`self.InstancedVisualItems`) 0 (`local.InstanceTransforms`) false true true))))